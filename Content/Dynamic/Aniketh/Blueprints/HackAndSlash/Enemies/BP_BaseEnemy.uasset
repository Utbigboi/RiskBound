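; Base enemy character for the hack-and-slash game, handling attacks, damage reactions and death.
; An enum state gates montage attacks and hit reactions, which are chosen by the damage type's direction or knock kind.
; A forward sphere trace damages the player once per swing, and a timeline lerp drives swept attack lunges.
; Death disables collision, plays a montage, adds player score and destroys the actor after a delay.
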(event `AttackKnockForce`
  (params (Distance :type "Float (single-precision)"))
  (bind _returnvalue (`self.K2_GetActorLocation`))
  ;[0.149 0.1263 0.04136 0.502] Add Forward Force While Attacking To Get Distance while Attacking
  (`self.StopKnockForce`)
  (if (!= Distance 0.0)
    (bind (_direction _alpha) (`Timeline|Timeline` :!label _label)
      (:`Update`
        (`self.K2_SetActorLocation` (`KismetMathLibrary.VLerp` (+ (* (`self.GetActorForwardVector`) Distance) _returnvalue) _returnvalue _alpha) true)))))

(event `StopKnockForce`
  ;[0.149 0.1263 0.04136 0.502] Add Forward Force While Attacking To Get Distance while Attacking
  (goto _label :!via `Stop`))

(event `self.ReceiveAnyDamage`
  (params (Damage :type "Float (single-precision)") (DamageType :type "DamageType Object Reference") (InstigatedBy :type "Controller Object Reference") (DamageCauser :type "Actor Object Reference"))
  (bind _output_get (set `self.Health` (- (`self.Health`) Damage)))
  (if (> _output_get 0.0)
    (bind _asbp_damage_type (cast `/Game/Dynamic/Aniketh/Blueprints/HackAndSlash/Damage_Type/BP_DamageType` DamageType))
    (bind _return_value (`self.GetHitReaction` (`/Game/Dynamic/Aniketh/Blueprints/HackAndSlash/Damage_Type/BP_DamageType.DamageType` _asbp_damage_type)))
    (if (and (`KismetSystemLibrary.IsValid` _return_value) (not (`self.IsCurrentStateEqualToAny` (`|MakeArray` "NewEnumerator3" :!type "/Game/Dynamic/Aniketh/Blueprints/HackAndSlash/Enums/E_States Enum"))))
      (`self.SetState` "NewEnumerator4")
      (`self.PlayAnimMontage` _return_value))
    (else
      (`self.PerformDeath`)
      (bind _asbp_hack_and_slash_character_aniket (cast `/Game/Dynamic/Aniketh/Blueprints/HackAndSlash/BP_HackAndSlashCharacterAniket` (`GameplayStatics.GetPlayerCharacter` 0)))
      (bind _output_get_2 (set `/Game/Dynamic/Aniketh/Blueprints/HackAndSlash/BP_HackAndSlashCharacterAniket.PlayerScore` (+ (`/Game/Dynamic/Aniketh/Blueprints/HackAndSlash/BP_HackAndSlashCharacterAniket.PlayerScore` _asbp_hack_and_slash_character_aniket) 100) _asbp_hack_and_slash_character_aniket))
      (`KismetSystemLibrary.PrintString` (`KismetStringLibrary.Conv_IntToString` _output_get_2))
      (`KismetSystemLibrary.Delay` 2.0)
      (`self.K2_DestroyActor`))))

(event `ResetState`
  (`self.SetState` "NewEnumerator0"))

(fn `CanAttack`
  (returns (`Return Value` :type Boolean))
  (bind _charactermovement (`self.CharacterMovement`))
  (return (and (not (`self.IsCurrentStateEqualToAny` (`|MakeArray` "NewEnumerator1" "NewEnumerator2" "NewEnumerator3" "NewEnumerator4" :!type "/Game/Dynamic/Aniketh/Blueprints/HackAndSlash/Enums/E_States Enum"))) (not (or (`NavMovementInterface.IsFlying` _charactermovement) (`NavMovementInterface.IsFalling` _charactermovement))))))

(fn `DrawEnemyColllision`
  (params (Radius :type "Float (single-precision)") (End :type "Float (single-precision)") (Damage :type "Float (double-precision)") (DamageTypeClass :type "DamageType Class Reference"))
  (bind _returnvalue (`self.K2_GetActorLocation`))
  (bind _returnvalue_2 (* (`self.BaseMobDamage`) (`self.DamageMultiplier`)))
  (`KismetArrayLibrary.Array_Clear` (`self.HitActors`))
  (set `self.DamageMultiplier` Damage)
  ; Colllision
  (bind (_outhits _returnvalue_3) (`KismetSystemLibrary.SphereTraceMultiForObjects` _returnvalue (+ (* (`self.GetActorForwardVector`) End) _returnvalue) Radius (`|MakeArray` "ObjectTypeQuery3" :!type "EObjectTypeQuery Enum")))
  (if _returnvalue_3
    ; Check Each Actor Hit
    (for _array_element _outhits
      (bind (_bblockinghit _binitialoverlap _time _distance _location _impactpoint _normal _impactnormal _physmat _hitactor) (`GameplayStatics.BreakHitResult` _array_element))
      (if (and (not (`KismetArrayLibrary.Array_Contains` (`self.HitActors`) _hitactor)) (`KismetSystemLibrary.IsValid` _hitactor))
        (bind _asbp_hack_and_slash_character_aniket (cast `/Game/Dynamic/Aniketh/Blueprints/HackAndSlash/BP_HackAndSlashCharacterAniket` _hitactor))
        (if (`|EnumInequality` (`/Game/Dynamic/Aniketh/Blueprints/HackAndSlash/BP_HackAndSlashCharacterAniket.GetState` _asbp_hack_and_slash_character_aniket) "NewEnumerator3")
          (`GameplayStatics.ApplyDamage` _hitactor _returnvalue_2 (`self.GetController` self) self (`local.DamageTypeClass`))
          (`/Game/Dynamic/Aniketh/Blueprints/HackAndSlash/BP_HackAndSlashCharacterAniket.TakeDamagePlayerEvent` _asbp_hack_and_slash_character_aniket _returnvalue_2)
          (`KismetArrayLibrary.Array_AddUnique` (`self.HitActors`) _hitactor))))))

(fn `GetEnemyCaspsuleCollider`
  (params (CapsuleComponentEnemy :type "CapsuleComponent Object Reference"))
  (set `self.CapsuleComponentEnemy` CapsuleComponentEnemy))

(fn `GetHitReaction`
  (params (`Damage Type` :type "/Game/Dynamic/Aniketh/Blueprints/HackAndSlash/Enums/E_DamageTypes Enum" :default "NewEnumerator0"))
  (returns (`Return Value` :type "AnimMontage Object Reference"))
  (switch `/Game/Dynamic/Aniketh/Blueprints/HackAndSlash/Enums/E_DamageTypes` `Damage Type`
    (:`NewEnumerator1`
      (return (`self.HR_R`)))
    (:`NewEnumerator2`
      (return (`self.HR_L`)))
    (:`NewEnumerator3`
      (return (`self.HR_Mid`)))
    (:`NewEnumerator4`
      (return (`self.HR_KnockDown`)))
    (:`NewEnumerator5`
      (return (`self.HR_KnockBack`)))))

(fn `GetState`
  (returns (`Return Value` :type "/Game/Dynamic/Aniketh/Blueprints/HackAndSlash/Enums/E_States Enum"))
  (return (`self.CurrentState`)))

(fn `IsCurrentStateEqualToAny`
  (params (StatesToCheck :type "Array of /Game/Dynamic/Aniketh/Blueprints/HackAndSlash/Enums/E_States Enum (by ref)"))
  (returns (ReturnValue :type Boolean))
  (return (`KismetArrayLibrary.Array_Contains` StatesToCheck (`self.CurrentState`))))

(fn `PerformAttack`
  (params (Index :type Integer))
  (returns (ReturnValue :type "Float (single-precision)"))
  (bind _output (`|GetArrayItem` (`self.AttackMontage`) Index))
  (if (`self.CanAttack`)
    (`/Engine/EditorBlueprintResources/StandardMacros.IsValid` _output
      (:`Is Valid`
        (`self.SetState` "NewEnumerator1")
        (bind _returnvalue (`AnimInstance.Montage_Play` (`SkeletalMeshComponent.GetAnimInstance` (`self.Mesh`)) _output 1.0 "MontageLength" 0.0 true))
        (return _returnvalue))
      (:`Is Not Valid`
        (return 0.0)))
    (else
      (return 0.0))))

(fn `PerformDeath`
  (`self.SetState` "NewEnumerator3")
  (`self.PlayAnimMontage` (`self.DeathMontage`))
  (`PrimitiveComponent.SetCollisionEnabled` (`self.CapsuleComponent`) "NoCollision")
  (`PrimitiveComponent.SetCollisionEnabled` (`self.Mesh`) "NoCollision"))

(fn `SetState`
  (params (NewState :type "/Game/Dynamic/Aniketh/Blueprints/HackAndSlash/Enums/E_States Enum" :default "NewEnumerator0"))
  (if (`|EnumInequality` NewState (`self.CurrentState`))
    (set `self.CurrentState` NewState)))

(fn `UserConstructionScript`)