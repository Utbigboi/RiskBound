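; Base AI controller for hack-and-slash enemies that runs each enemy's behavior tree and periodically triggers attacks.
; On possessing a BP_BaseEnemy, it starts that pawn's tree and seeds the blackboard with the player character as target and a strafe distance.
; A looping timer, its interval randomized once at possession, sets the blackboard's behavior state and attack flag, leaving execution to the tree.
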(event `PerformAttack`
  (bind _returnvalue (`AIBlueprintHelperLibrary.GetBlackboard` self))
  (`/Engine/EditorBlueprintResources/StandardMacros.IsValid` _returnvalue
    (:`Is Valid`
      (`BlackboardComponent.SetValueAsEnum` _returnvalue (`self.StateKeyName`) (cast `/Game/Dynamic/Aniketh/Blueprints/HackAndSlash/Enums/E_BehaviorStates` (enumliteral `/Game/Dynamic/Aniketh/Blueprints/HackAndSlash/Enums/E_BehaviorStates` "NewEnumerator3")))
      (`BlackboardComponent.SetValueAsBool` _returnvalue (`self.SaveAttackKeyName`) true))))

(event `self.ReceivePossess`
  (params (PossessedPawn :type "Pawn Object Reference"))
  (bind _asbp_base_enemy (cast `/Game/Dynamic/Aniketh/Blueprints/HackAndSlash/Enemies/BP_BaseEnemy` PossessedPawn))
  (`self.RunBehaviorTree` self (`/Game/Dynamic/Aniketh/Blueprints/HackAndSlash/Enemies/BP_BaseEnemy.BehaviorTree` _asbp_base_enemy))
  (`self.SetBlackboardKey`)
  (`KismetSystemLibrary.K2_SetTimerDelegate` (delegate `PerformAttack`) (`KismetMathLibrary.RandomFloatInRange` 3.0 8.0) true))

(fn `SetBlackboardKey`
  (bind _returnvalue (`AIBlueprintHelperLibrary.GetBlackboard` self))
  (`/Engine/EditorBlueprintResources/StandardMacros.IsValid` _returnvalue
    (:`Is Valid`
      (`BlackboardComponent.SetValueAsObject` _returnvalue (`self.TargetKeyName`) (`GameplayStatics.GetPlayerCharacter` 0))
      (`BlackboardComponent.SetValueAsFloat` _returnvalue (`self.StrafeDistanceKeyName`) (`self.StrafeDistance`)))))

(fn `UserConstructionScript`)