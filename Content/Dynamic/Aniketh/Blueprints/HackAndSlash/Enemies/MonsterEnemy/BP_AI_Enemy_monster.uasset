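; Monster enemy character for a hack-and-slash game that attacks the player and awards score when killed.
; Pawn sensing sets a blackboard flag for the AI, and AttackPlayer plays an attack montage when a forward sphere trace finds the living player.
; DrawEnemyMonsterCollision multi-traces to damage the player once per hit, skipping one player state, with base damage raised by IncreaseDifficulty.
; AnyDamage plays hit or death montages, then fires OnDeath and destroys the actor.
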(event `IncreaseDifficulty`
  (set `self.BaseMonsterDamage` (* (`self.BaseMonsterDamage`) 1.2)))

(event `self.PawnSensing.OnSeePawn`
  (params (Pawn :type "Pawn Object Reference"))
  (cast `/Game/Dynamic/Aniketh/Blueprints/HackAndSlash/BP_HackAndSlashCharacterAniket` Pawn)
  (`BlackboardComponent.SetValueAsBool` (`AIBlueprintHelperLibrary.GetBlackboard` (`AIBlueprintHelperLibrary.GetAIController` self)) "hasSeenPlayer" true))

(event `Attack Player`
  (bind _returnvalue (`self.K2_GetActorLocation`))
  (bind _asbp_hack_and_slash_character_aniket (cast `/Game/Dynamic/Aniketh/Blueprints/HackAndSlash/BP_HackAndSlashCharacterAniket` (`GameplayStatics.GetPlayerCharacter` 0)))
  (if (not (`/Game/Dynamic/Aniketh/Blueprints/HackAndSlash/BP_HackAndSlashCharacterAniket.IsPlayerDead` _asbp_hack_and_slash_character_aniket))
    (bind (_outhit _returnvalue_2) (`KismetSystemLibrary.SphereTraceSingleForObjects` _returnvalue (+ _returnvalue (* (`KismetMathLibrary.GetForwardVector` (`self.K2_GetActorRotation`)) 250.0)) 120.0 (`|MakeArray` "ObjectTypeQuery3" :!type "EObjectTypeQuery Enum")))
    (if _returnvalue_2
      (cast `/Game/Dynamic/Aniketh/Blueprints/HackAndSlash/BP_HackAndSlashCharacterAniket` (`.HitActor` (`GameplayStatics.BreakHitResult` _outhit)))
      (`self.PlayAnimMontage` "/Game/Static/FourEvilDragonsHP/Animations/DragonTheNightmare/AM_AttackHand.AM_AttackHand"))))

(event `self.ReceiveAnyDamage`
  (params (Damage :type "Float (single-precision)") (DamageType :type "DamageType Object Reference") (InstigatedBy :type "Controller Object Reference") (DamageCauser :type "Actor Object Reference"))
  (bind _output_get (set `self.Health` (- (`self.Health`) Damage)))
  (if (> _output_get 0.0)
    (`self.PlayAnimMontage` "/Game/Static/FourEvilDragonsHP/Animations/DragonTheNightmare/AM_MonsterHitReaction.AM_MonsterHitReaction")
    (else
      (set `self.isMonsterDead` true)
      (`self.PlayAnimMontage` "/Game/Static/FourEvilDragonsHP/Animations/DragonTheNightmare/AM_MonsterDie.AM_MonsterDie")
      (`PrimitiveComponent.SetCollisionEnabled` (`self.CapsuleComponent`) "NoCollision")
      (`PrimitiveComponent.SetCollisionEnabled` (`self.Capsule`) "NoCollision")
      (`PrimitiveComponent.SetCollisionEnabled` (`self.Mesh`) "NoCollision")
      (bind _asbp_hack_and_slash_character_aniket (cast `/Game/Dynamic/Aniketh/Blueprints/HackAndSlash/BP_HackAndSlashCharacterAniket` (`GameplayStatics.GetPlayerCharacter` 0)))
      (bind _output_get_2 (set `/Game/Dynamic/Aniketh/Blueprints/HackAndSlash/BP_HackAndSlashCharacterAniket.PlayerScore` (+ (`/Game/Dynamic/Aniketh/Blueprints/HackAndSlash/BP_HackAndSlashCharacterAniket.PlayerScore` _asbp_hack_and_slash_character_aniket) 200) _asbp_hack_and_slash_character_aniket))
      (`KismetSystemLibrary.PrintString` (`KismetStringLibrary.Conv_IntToString` _output_get_2))
      (`KismetSystemLibrary.Delay` 2.0)
      (`self.OnDeath`)
      (`self.K2_DestroyActor`))))

(fn `DrawEnemyMonsterCollision`
  (params (Radius :type "Float (single-precision)") (End :type "Float (single-precision)") (Damage :type "Float (double-precision)") (DamageTypeClass :type "/Game/Dynamic/Aniketh/Blueprints/HackAndSlash/Damage_Type/BP_DamageType Class Reference"))
  (bind _returnvalue (`self.K2_GetActorLocation`))
  (bind _returnvalue_2 (* (`self.DamageMultiplier`) (`self.BaseMonsterDamage`)))
  (`KismetArrayLibrary.Array_Clear` (`self.HitActors`))
  (set `self.DamageMultiplier` Damage)
  ; Colllision
  (bind (_outhits _returnvalue_3) (`KismetSystemLibrary.SphereTraceMultiForObjects` _returnvalue (+ (* (`self.GetActorForwardVector`) End) _returnvalue) Radius (`|MakeArray` "ObjectTypeQuery3" :!type "EObjectTypeQuery Enum")))
  (if _returnvalue_3
    ; Check Each Actor Hit
    (for _array_element _outhits
      (bind (_bblockinghit _binitialoverlap _time _distance _location _impactpoint _normal _impactnormal _physmat _hitactor) (`GameplayStatics.BreakHitResult` _array_element))
      (if (and (not (`KismetArrayLibrary.Array_Contains` (`self.HitActors`) _hitactor)) (`KismetSystemLibrary.IsValid` _hitactor))
        (bind _asbp_hack_and_slash_character_aniket (cast `/Game/Dynamic/Aniketh/Blueprints/HackAndSlash/BP_HackAndSlashCharacterAniket` _hitactor))
        (if (`|EnumInequality` (`/Game/Dynamic/Aniketh/Blueprints/HackAndSlash/BP_HackAndSlashCharacterAniket.GetState` _asbp_hack_and_slash_character_aniket) "NewEnumerator3")
          (`GameplayStatics.ApplyDamage` _hitactor _returnvalue_2 (`self.GetController` self) self (`self.DamageTypeClass`))
          (`/Game/Dynamic/Aniketh/Blueprints/HackAndSlash/BP_HackAndSlashCharacterAniket.TakeDamagePlayerEvent` _asbp_hack_and_slash_character_aniket _returnvalue_2)
          (`KismetArrayLibrary.Array_AddUnique` (`self.HitActors`) _hitactor))))))

(fn `UserConstructionScript`)