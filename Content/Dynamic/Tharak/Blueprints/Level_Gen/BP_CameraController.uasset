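; Camera actor that becomes the first player's view target on BeginPlay and moves between given locations and rotations.
; MoveCam stores the current and target transforms, then plays the CamLerp timeline to interpolate location and rotation.
; MoveCameraTo instead snaps the actor straight to a target location and rotation.
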(event `self.ReceiveBeginPlay`
  (`PlayerController.SetViewTargetWithBlend` (`GameplayStatics.GetPlayerController` 0) self 0.0 "VTBlend_Linear" 0.0 false))

(event `MoveCam`
  (params (TargetLocation :type "Vector Structure") (TargetRotation :type "Rotator Structure"))
  (set `self.StartLocation` (`self.K2_GetActorLocation`))
  (set `self.StartRotation` (`self.K2_GetActorRotation`))
  (set `self.EndLocation` TargetLocation)
  (set `self.EndRotation` TargetRotation)
  (bind (_direction _alpha) (`Timeline|CamLerp` :!via `PlayFromStart`)
    (:`Update`
      (`self.K2_SetActorLocationAndRotation` (`KismetMathLibrary.VLerp` (`self.StartLocation`) (`self.EndLocation`) _alpha) (`KismetMathLibrary.RLerp` (`self.StartRotation`) (`self.EndRotation`) _alpha)))))

(fn `MoveCameraTo`
  (params (TargetLocation :type "Vector Structure") (TargetRotation :type "Rotator Structure"))
  (`self.K2_SetActorLocationAndRotation` TargetLocation TargetRotation))

(fn `UserConstructionScript`)