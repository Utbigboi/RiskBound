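; BP_Dungeon_Gen is a procedural dungeon generator that builds a layout from room actors on BeginPlay.
; It spawns BP_Dungeon_Room1 at its own transform and gathers the children of that room's ExitFolder into ExitsList.
; SpawnNextRoom consumes a random exit, spawns a random RoomList class there and adds the new room's exits.
; It calls itself recursively until RoomAmount runs out, with no overlap check.
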(event `Spawn Start Room`
  ;[0 0.7135 0.08749 0.5 20] Spawn Start Room
  (bind _returnvalue (`|SpawnActorFromClass` "/Game/Dynamic/Tharak/Blueprints/Level_Gen/BP_Dungeon_Room1.BP_Dungeon_Room1_C" (`SceneComponent.K2_GetComponentToWorld` (`self.DefaultSceneRoot`)) "AlwaysSpawn" "MultiplyWithRoot" null null))
  (`KismetArrayLibrary.Array_Append` (`self.ExitsList`) (`SceneComponent.GetChildrenComponents` (`/Game/Dynamic/Tharak/Blueprints/Level_Gen/BP_Master_Room.ExitFolder` _returnvalue) false)))

(event `Spawn Next Room`
  ;[0 0.6771 0.06874 0.5 20] Spawn Next Room
  (bind _output_get (set `self.Selected Exit Point` (`KismetArrayLibrary.Array_Random` (`self.ExitsList`))))
  (`KismetArrayLibrary.Array_RemoveItem` (`self.ExitsList`) _output_get)
  (bind _returnvalue (`|SpawnActorFromClass` (`KismetArrayLibrary.Array_Random` (`self.Room List`)) (`SceneComponent.K2_GetComponentToWorld` (`self.Selected Exit Point`)) "AlwaysSpawn" "MultiplyWithRoot" null null))
  (bind _asbp_master_room (cast `/Game/Dynamic/Tharak/Blueprints/Level_Gen/BP_Master_Room` _returnvalue))
  (set `self.Latest Room` _asbp_master_room)
  (`KismetArrayLibrary.Array_Append` (`self.ExitsList`) (`SceneComponent.GetChildrenComponents` (`/Game/Dynamic/Tharak/Blueprints/Level_Gen/BP_Master_Room.ExitFolder` (`self.Latest Room`)) false))
  (set `self.Room Amount` (- (`self.Room Amount`) 1))
  (if (> (`self.Room Amount`) 0)
    (`self.Spawn Next Room`)))

(event `self.ReceiveBeginPlay`
  (`self.Spawn Start Room`)
  (`self.Spawn Next Room`))

(fn `UserConstructionScript`)