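; BP_Master_Room is a room actor for level generation, with a double door and its own camera anchor.
; When the hack-and-slash character enters RoomTrigger, it moves the camera controller to that anchor and increments the game mode's IncreaseAdditioner, printing the value.
; The Door event plays a timeline that rotates both door meshes, and an Exit overlap by any actor reverses it.
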(event `DoorOpen`
  (bind (_direction _door _door2) (`Timeline|DoorRotation` :!label _label)
    (:`Update`
      (`SceneComponent.K2_SetRelativeLocationAndRotation` (`self.Door_2Side_SM`) (2750.0 -150.0 0.0) (`KismetMathLibrary.MakeRotator` 0.0 0.0 _door) false false)
      (`SceneComponent.K2_SetRelativeLocationAndRotation` (`self.Door_2Side_SM1`) (2750.0 150.0 0.0) (`KismetMathLibrary.MakeRotator` 0.0 0.0 _door2) false false))))

(event `self.Exit.OnComponentBeginOverlap`
  (params (OverlappedComponent :type "PrimitiveComponent Object Reference") (OtherActor :type "Actor Object Reference") (OtherComp :type "PrimitiveComponent Object Reference") (OtherBodyIndex :type Integer) (bFromSweep :type Boolean) (SweepResult :type "HitResult Structure (by ref)"))
  (goto _label :!via `Reverse`))

(event `/Game/Dynamic/Tharak/Blueprints/BPI_InteractInterface.Door`
  (`self.DoorOpen`))

(event `self.Room Trigger.OnComponentBeginOverlap`
  (params (OverlappedComponent :type "PrimitiveComponent Object Reference") (OtherActor :type "Actor Object Reference") (OtherComp :type "PrimitiveComponent Object Reference") (OtherBodyIndex :type Integer) (bFromSweep :type Boolean) (SweepResult :type "HitResult Structure (by ref)"))
  (bind _cameraanchor (`self.CameraAnchor`))
  (cast `/Game/Dynamic/Aniketh/Blueprints/HackAndSlash/BP_HackAndSlashCharacterAniket` OtherActor)
  (bind _returnvalue (`GameplayStatics.GetActorOfClass` "/Game/Dynamic/Tharak/Blueprints/Level_Gen/BP_CameraController.BP_CameraController_C"))
  (`/Game/Dynamic/Tharak/Blueprints/Level_Gen/BP_CameraController.MoveCam` _returnvalue (`SceneComponent.K2_GetComponentLocation` _cameraanchor) (`SceneComponent.K2_GetComponentRotation` _cameraanchor))
  (bind _asbp_aniketh_game_mode (cast `/Game/Dynamic/Aniketh/Blueprints/BP_AnikethGameMode` (`GameplayStatics.GetGameMode`)))
  (bind _output_get (set `/Game/Dynamic/Aniketh/Blueprints/BP_AnikethGameMode.IncreaseAdditioner` (+ (`/Game/Dynamic/Aniketh/Blueprints/BP_AnikethGameMode.IncreaseAdditioner` _asbp_aniketh_game_mode) 1) _asbp_aniketh_game_mode))
  (`KismetSystemLibrary.PrintString` (`KismetStringLibrary.Conv_IntToString` _output_get)))

(fn `UserConstructionScript`)