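; Blueprint function library that rolls dice and turns the result into a Health, Damage or Speed modifier on an actor stats struct.
; The main roll function handles the Strait roll type, summing random rolls of the chosen die size and returning the total with the stats.
; Totals 1–3 halve one stat and 4–6 double one; higher totals have no case.
; The result modifier input is unused, and PlayerStats is a pass-through.
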(fn `BFL_DIceResultMod`
  (params (Result :type Integer))
  (returns (Stats :type "/Game/Dynamic/Maheesh/BluePrints/Struct_ActorStats Structure"))
  (locals (ResultLocal :type Integer) (TypeLocal :type Integer) (ActorStats :type "/Game/Dynamic/Maheesh/BluePrints/Struct_ActorStats Structure") (Health :type Integer :default 50) (Damage :type Integer :default 25) (Speed :type Integer :default 200))
  (bind (_actorstats_health _actorstats_speed _actorstats_damage) (break `/Game/Dynamic/Maheesh/BluePrints/Struct_ActorStats` (`local.ActorStats`)))
  (bind (_actorstats_health_2 _actorstats_speed_2 _actorstats_damage_2) (break `/Game/Dynamic/Maheesh/BluePrints/Struct_ActorStats` (`local.ActorStats`)))
  (if (< Result 4)
    (switch `int` Result
      (:`1`
        (set `local.Health` (/ _actorstats_health_2 2)))
      (:`2`
        (set `local.Damage` (/ _actorstats_damage_2 2)))
      (:`3`
        (set `local.Speed` (/ _actorstats_speed_2 2))))
    (else
      (switch `int` Result
        (:`4`
          (set `local.Health` (* _actorstats_health 2)))
        (:`5`
          (set `local.Damage` (* _actorstats_damage 2)))
        (:`6`
          (set `local.Speed` (* _actorstats_speed 2))))))
  (bind _output_get (set `local.ActorStats` (make `/Game/Dynamic/Maheesh/BluePrints/Struct_ActorStats` (`local.Health`) (`local.Speed`) (`local.Damage`))))
  (return _output_get))

(fn `BFL_DiceRoll`
  (params (Dice :type Integer) (AmountToRoll :type Integer) (NewParam :type "/Game/Dynamic/Maheesh/BluePrints/Enum_RollType Enum" :default "NewEnumerator0") (`ResultModifer(+/-)` :type Integer))
  (returns (Result :type Integer) (Stats :type "/Game/Dynamic/Maheesh/BluePrints/Struct_ActorStats Structure"))
  (locals (DiceTypeLocal :type Integer :default 6) (AmounttoRollLocal :type Integer) (ResultModLocal :type Integer) (RollTypeLocal :type "/Game/Dynamic/Maheesh/BluePrints/Enum_RollType Enum" :default "NewEnumerator0"))
  (set `local.DiceTypeLocal` Dice)
  (set `local.AmounttoRollLocal` AmountToRoll)
  (set `local.RollTypeLocal` NewParam)
  (set `local.ResultModLocal` `ResultModifer(+/-)`)
  (switch `/Game/Dynamic/Maheesh/BluePrints/Enum_RollType` (`local.RollTypeLocal`)
    (:`NewEnumerator0`
      (bind _result (`self.BFL_NEST_StraitRoll` (`local.DiceTypeLocal`) (`local.AmounttoRollLocal`)))
      (bind _stats (`self.BFL_DIceResultMod` _result))
      (bind _playerstats (`self.BFL_PlayerStats` _stats))
      (return _result _playerstats))))

(fn `BFL_NEST_StraitRoll`
  (params (DiceType :type Integer) (Amount :type Integer))
  (returns (Result :type Integer))
  (locals (ResultLocal :type Integer))
  (for _ (range 1 (+ Amount 1))
    (set `local.ResultLocal` (+ (`KismetMathLibrary.RandomIntegerInRange` 1 DiceType) (`local.ResultLocal`))))
  (return (`local.ResultLocal`)))

(fn `BFL_PlayerStats`
  (params (ps :type "/Game/Dynamic/Maheesh/BluePrints/Struct_ActorStats Structure"))
  (returns (PlayerStats :type "/Game/Dynamic/Maheesh/BluePrints/Struct_ActorStats Structure"))
  (return ps))